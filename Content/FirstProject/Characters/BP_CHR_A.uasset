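; BP_CHR_A is a player-controllable Character Blueprint that handles basic look, move, sprint and jump input.
; Turn and LookUp axes feed controller yaw and pitch, while the move axes drive movement along the actor's own forward and right vectors.
; Holding Sprint directly raises CharacterMovement's max walk speed, and releasing it sets a fixed normal speed.
; Jump triggers on press with no release handling, and the construction script is empty.
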(event `InputAxis|Turn`
  (params (AxisValue :type "Float (single-precision)"))
  ;[1 1 1] Входные данные
  (`self.AddControllerYawInput` AxisValue))

(event `InputAxis|LookUp`
  (params (AxisValue :type "Float (single-precision)"))
  ;[1 1 1] Входные данные
  (`self.AddControllerPitchInput` AxisValue))

(event `InputAxis|MoveForward`
  (params (AxisValue :type "Float (single-precision)"))
  ;[1 1 1] Входные данные
  (`self.AddMovementInput` (`self.GetActorForwardVector`) AxisValue))

(event `InputAxis|MoveRight`
  (params (AxisValue :type "Float (single-precision)"))
  ;[1 1 1] Входные данные
  (`self.AddMovementInput` (`self.GetActorRightVector`) AxisValue))

(event `InputAction|Interact`
  (params (Key :type "Key Structure"))
  ;[1 1 1] Входные данные
)

(event `InputAction|Sprint`
  (params (Key :type "Key Structure"))
  ;[1 1 1] Входные данные
  (:`Pressed`
    (set `CharacterMovementComponent.MaxWalkSpeed` 3000.0 (`self.CharacterMovement`)))
  (:`Released`
    (set `CharacterMovementComponent.MaxWalkSpeed` 600.0 (`self.CharacterMovement`))))

(event `InputAction|Jump`
  (params (Key :type "Key Structure"))
  ;[1 1 1] Входные данные
  (:`Pressed`
    (`self.Jump`)))

(fn `UserConstructionScript`)