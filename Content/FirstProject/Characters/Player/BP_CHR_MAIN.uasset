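; Main player character with first/third-person style movement input, sprinting, single-weapon handling and death.
; Capsule overlap tracks a nearby Gun, which Interact attaches to WeaponPlace, replacing any held weapon; Fire and Drop act on it.
; Sprint changes walk speed and starts self-recalling delayed events that drain or regenerate stamina.
; Damage feeds StatusAC, whose OnDeath ragdolls the mesh with a head impulse along the last point-damage direction.
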(event `self.CapsuleComponent.OnComponentBeginOverlap`
  (params (OverlappedComponent :type "PrimitiveComponent Object Reference") (OtherActor :type "Actor Object Reference") (OtherComp :type "PrimitiveComponent Object Reference") (OtherBodyIndex :type Integer) (bFromSweep :type Boolean) (SweepResult :type "HitResult Structure (by ref)"))
  (`|ExecutionSequence`
    (:`then_0`
      (bind _asgun (cast `/Game/FirstProject/Content/Weapon/Weapons/Gun` OtherActor))
      (set `self.Interact Gun` _asgun))
    (:`then_1`
      (cast `/Game/FirstProject/Interactions/InteractBase` OtherActor))))

(event `self.CapsuleComponent.OnComponentEndOverlap`
  (params (OverlappedComponent :type "PrimitiveComponent Object Reference") (OtherActor :type "Actor Object Reference") (OtherComp :type "PrimitiveComponent Object Reference") (OtherBodyIndex :type Integer))
  (if (== OtherActor (`self.Interact Gun`))
    (set `self.Interact Gun` null)))

(event `Drain Stamina`
  ;[1 1 1] Stamina
  (bind _output_get (set `self.Stamina` (`KismetMathLibrary.FClamp` (- (`self.Stamina`) 5.0) 0.0 (`self.Max Stamina`))))
  (if (== _output_get 0.0)
    (`self.Stop Sprinting`)
    (elif (`self.Sprinting?`)
      (`KismetSystemLibrary.Delay` 1.0)
      (`self.Drain Stamina`))))

(event `self.ReceiveAnyDamage`
  (params (Damage :type "Float (single-precision)") (DamageType :type "DamageType Object Reference") (InstigatedBy :type "Controller Object Reference") (DamageCauser :type "Actor Object Reference"))
  (`/Game/FirstProject/Characters/Player/StatusAC.MakeDamage/Health` (`self.StatusAC`) Damage))

(event `Regen Stamina`
  ;[1 1 1] Stamina
  (bind _output_get (set `self.Stamina` (`KismetMathLibrary.FClamp` (+ (`self.Stamina`) 5.0) 0.0 (`self.Max Stamina`))))
  (if (== _output_get (`self.Max Stamina`))
    _
    (elif (not (`self.Sprinting?`))
      (`KismetSystemLibrary.Delay` 1.0)
      (`self.Regen Stamina`))))

(event `self.ReceivePointDamage`
  (params (Damage :type "Float (single-precision)") (DamageType :type "DamageType Object Reference") (HitLocation :type "Vector Structure") (HitNormal :type "Vector Structure") (HitComponent :type "PrimitiveComponent Object Reference") (BoneName :type Name) (ShotFromDirection :type "Vector Structure") (InstigatedBy :type "Controller Object Reference") (DamageCauser :type "Actor Object Reference") (HitInfo :type "HitResult Structure (by ref)"))
  (set `self.Last Point Damage Direction` ShotFromDirection))

(event `self.StatusAC.OnDeath`
  ;[1 1 1] Обработка смерти
  (`/Engine/EditorBlueprintResources/StandardMacros.DoOnce` false
    (:`Completed`
      (`PrimitiveComponent.SetSimulatePhysics` (`self.Mesh`) true)
      (`KismetSystemLibrary.Delay` 0.0)
      (`PrimitiveComponent.AddImpulse` (`self.Mesh`) (* (`self.Last Point Damage Direction`) (`self.Impulse`)) "Head" true)
      (`ActorComponent.K2_DestroyComponent` (`self.CapsuleComponent`)))))

(event `InputAxis|Turn`
  (params (AxisValue :type "Float (single-precision)"))
  ;[1 1 1] Входные данные
  (`self.AddControllerYawInput` AxisValue))

(event `InputAxis|LookUp`
  (params (AxisValue :type "Float (single-precision)"))
  ;[1 1 1] Входные данные
  (`self.AddControllerPitchInput` AxisValue))

(event `InputAxis|MoveForward`
  (params (AxisValue :type "Float (single-precision)"))
  ;[1 1 1] Входные данные
  (`self.AddMovementInput` (`self.GetActorForwardVector`) AxisValue))

(event `InputAxis|MoveRight`
  (params (AxisValue :type "Float (single-precision)"))
  ;[1 1 1] Входные данные
  (`self.AddMovementInput` (`self.GetActorRightVector`) AxisValue))

(event `InputAction|Interact`
  (params (Key :type "Key Structure"))
  ;[1 1 1] Входные данные
  (:`Pressed`
    (`|ExecutionSequence`
      (:`then_0`
        (if (`KismetSystemLibrary.IsValid` (`self.Interact Gun`))
          (`self.Take Weapon`))))))

(event `InputAction|Fire`
  (params (Key :type "Key Structure"))
  (bind _active_weapon (`self.Active Weapon`))
  ;[1 1 1] Входные данные
  (:`Pressed`
    (if (`KismetSystemLibrary.IsValid` _active_weapon)
      (`/Game/FirstProject/Content/Weapon/Weapons/WeaponBase.Fire` _active_weapon))))

(event `InputAction|Drop Weapon`
  (params (Key :type "Key Structure"))
  ;[1 1 1] Входные данные
  (:`Pressed`
    (`self.Drop Weapon`)))

(event `InputAction|Sprint`
  (params (Key :type "Key Structure"))
  ;[1 1 1] Входные данные
  (:`Pressed`
    (`self.Start Sprint`))
  (:`Released`
    (`self.Stop Sprinting`)))

(event `InputAction|Jump`
  (params (Key :type "Key Structure"))
  ;[1 1 1] Входные данные
  (:`Pressed`
    (`self.Jump`)))

(fn `Drop Weapon`
  (if (`KismetSystemLibrary.IsValid` (`self.Active Weapon`))
    (`PrimitiveComponent.SetSimulatePhysics` (`/Game/FirstProject/Content/Weapon/Weapons/WeaponBase.StaticMesh` (`self.Active Weapon`)) true)
    (`PrimitiveComponent.SetCollisionEnabled` (`/Game/FirstProject/Content/Weapon/Weapons/WeaponBase.StaticMesh` (`self.Active Weapon`)) "QueryAndPhysics")
    (`self.K2_DetachFromActor` (`self.Active Weapon`) "KeepWorld" "KeepWorld" "KeepRelative")
    (set `self.Active Weapon` null)))

(fn `Start Sprint`
  (set `CharacterMovementComponent.MaxWalkSpeed` 900.0 (`self.CharacterMovement`))
  (set `self.Sprinting?` true)
  (`self.Drain Stamina`))

(fn `Stop Sprinting`
  (set `CharacterMovementComponent.MaxWalkSpeed` 600.0 (`self.CharacterMovement`))
  (set `self.Sprinting?` false)
  (`self.Regen Stamina`))

(fn `Take Weapon`
  (if (`KismetSystemLibrary.IsValid` (`self.Active Weapon`))
    (`self.Drop Weapon`))
  (bind _output_get (set `self.Active Weapon` (`self.Interact Gun`)))
  (`self.K2_AttachToComponent` _output_get (`self.Weapon place`) "None" "SnapToTarget" "SnapToTarget" "KeepRelative" true)
  (`PrimitiveComponent.SetCollisionEnabled` (`/Game/FirstProject/Content/Weapon/Weapons/WeaponBase.StaticMesh` (`self.Active Weapon`)) "NoCollision")
  (`PrimitiveComponent.SetSimulatePhysics` (`/Game/FirstProject/Content/Weapon/Weapons/WeaponBase.StaticMesh` (`self.Active Weapon`)) false)
  (set `self.Interact Gun` null))

(fn `UserConstructionScript`)