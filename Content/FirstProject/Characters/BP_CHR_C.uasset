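; BP_CHR_C is a player Character Blueprint that handles basic look, movement, sprint and jump input.
; Axis events drive controller yaw and pitch, and movement along the actor's forward and right vectors.
; Sprint switches CharacterMovement's max walk speed while held, and Jump calls the built-in jump.
; Interact only prints debug text, and debug prints also remain on strafe and jump.
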(event `InputAxis|Turn`
  (params (AxisValue :type "Float (single-precision)"))
  ;[1 1 1] Входные данные
  (`self.AddControllerYawInput` AxisValue))

(event `InputAxis|LookUp`
  (params (AxisValue :type "Float (single-precision)"))
  ;[1 1 1] Входные данные
  (`self.AddControllerPitchInput` AxisValue))

(event `InputAxis|MoveForward`
  (params (AxisValue :type "Float (single-precision)"))
  ;[1 1 1] Входные данные
  (`self.AddMovementInput` (`self.GetActorForwardVector`) AxisValue))

(event `InputAxis|MoveRight`
  (params (AxisValue :type "Float (single-precision)"))
  ;[1 1 1] Входные данные
  (`KismetSystemLibrary.PrintString` (`KismetStringLibrary.Conv_DoubleToString` AxisValue))
  (`self.AddMovementInput` (`self.GetActorRightVector`) AxisValue))

(event `InputAction|Interact`
  (params (Key :type "Key Structure"))
  ;[1 1 1] Входные данные
  (:`Pressed`
    (`KismetSystemLibrary.PrintString` "Pressed"))
  (:`Released`
    (`KismetSystemLibrary.PrintString` "Released")))

(event `InputAction|Sprint`
  (params (Key :type "Key Structure"))
  ;[1 1 1] Входные данные
  (:`Pressed`
    (set `CharacterMovementComponent.MaxWalkSpeed` 1450.0 (`self.CharacterMovement`)))
  (:`Released`
    (set `CharacterMovementComponent.MaxWalkSpeed` 750.0 (`self.CharacterMovement`))))

(event `InputAction|Jump`
  (params (Key :type "Key Structure"))
  ;[1 1 1] Входные данные
  (:`Pressed`
    (`KismetSystemLibrary.PrintString` "Jump")
    (`self.Jump`)))

(fn `UserConstructionScript`)